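; Jump component that adds a limited number of mid-air strafe dashes when jump is pressed while falling; grounded presses use the parent jump.
; Each dash locks direction from last movement input, or actor forward without input.
; Tick runs only during a dash, overriding velocity with curve-driven horizontal speed and constant upward speed until the curve ends, blocking further jumps meanwhile.
; The dash count resets on landing or through ResetStrafeCount.
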(event Custom|Reset%20StrafeCount
  (Variables|Private|SetStrafeCount 0))

(event EventBeginPlay
  (|CallParentFunction) ; This node is disabled and will not be called.\nDrag off pins to build functionality.
)

(event EventTick
  (params (DeltaSeconds :type Float%20%28single-precision%29))
  (Private|TickStrafe DeltaSeconds))

(fn Jump
  (if (not (Class|ActorComponent|IsComponentTickEnabled))
    (if (AI|Components|NavMovement|IsFalling (Variables|/Script/Engine.Character|GetCharacterMovement (CallFunction|GetOwningCharacter)))
      (if (< (Variables|Private|GetStrafeCount) (Variables|Private|GetMaxStrafes))
        (Math|Integer|IncrementInt (Variables|Private|GetStrafeCount)
          (:%20%20
            (Private|BeginStrafe))))
      (else
        (|CallParentFunction)))))

(fn StopJumping
  (|CallParentFunction))

(fn OnLanded
  (|CallParentFunction)
  (Variables|Private|SetStrafeCount 0))

(fn BeginStrafe
  (bind _owningcharacter (CallFunction|GetOwningCharacter))
  (bind _returnvalue (Class|Pawn|GetLastMovementInputVector _owningcharacter))
  (bind _returnvalue_2 (Math|Conversions|ToVector2D(Vector) _returnvalue))
  (bind _returnvalue_3 (Math|Vector2D|Normalize2D _returnvalue_2))
  (Components|Tick|SetComponentTickEnabled true)
  (Variables|Private|SetStrafeTimer (.MinTime (Math|Curves|GetTimeRange (Variables|Private|GetStrafeCurve))))
  (if (Class|KismetMathLibrary|IsZero2D _returnvalue_3)
    (Variables|Private|SetStrafeDerection (Math|Conversions|ToVector2D(Vector) (Transformation|GetActorForwardVector (CallFunction|GetOwningCharacter))))
    (else
      (Variables|Private|SetStrafeDerection _returnvalue_3))))

(fn EndStrafe
  (Components|Tick|SetComponentTickEnabled false))

(fn TickStrafe
  (params (DeltaSeconds :type Float%20%28single-precision%29))
  (bind _strafecurve (Variables|Private|GetStrafeCurve))
  (bind (_mintime _maxtime) (Math|Curves|GetTimeRange _strafecurve))
  (bind _output_get (Variables|Private|SetStrafeTimer (+ (Variables|Private|GetStrafeTimer) DeltaSeconds)))
  (if (Math|Float|InRange(Float) _output_get _mintime _maxtime)
    (Variables|/Script/Engine.MovementComponent|SetVelocity (Variables|/Script/Engine.Character|GetCharacterMovement (CallFunction|GetOwningCharacter)) (Math|Vector|MakeVector (.x (* (Variables|Private|GetStrafeDerection) (Math|Curves|GetFloatValue (Variables|Private|GetStrafeCurve) (Variables|Private|GetStrafeTimer)))) (.y (* (Variables|Private|GetStrafeDerection) (Math|Curves|GetFloatValue (Variables|Private|GetStrafeCurve) (Variables|Private|GetStrafeTimer)))) 1e+02))
    (else
      (Private|EndStrafe))))