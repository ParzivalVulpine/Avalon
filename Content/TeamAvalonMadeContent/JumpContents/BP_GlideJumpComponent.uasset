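; Jump component that adds a glide to the owning character's jump, limiting how fast it falls or loses vertical speed.
; Jump extends the parent behavior by starting a timer and enabling component tick when the character can jump.
; Each tick floors Z velocity to a float curve sampled at that timer, leaving horizontal velocity untouched.
; Releasing jump or leaving the curve's time range disables tick and ends the glide.
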(event EventBeginPlay
  (|CallParentFunction) ; This node is disabled and will not be called.\nDrag off pins to build functionality.
)

(event EventTick
  (params (DeltaSeconds :type Float%20%28single-precision%29))
  (Private|TickGlide DeltaSeconds))

(fn Jump
  (if (Character|CanJump (CallFunction|GetOwningCharacter))
    (|CallParentFunction)
    (Private|BeginGlide)))

(fn BeginGlide
  (Components|Tick|SetComponentTickEnabled true)
  (Variables|Default|SetGlideTimer (.MinTime (Math|Curves|GetTimeRange (Variables|Private|GetGlideCurve)))))

(fn EndGlide
  (Components|Tick|SetComponentTickEnabled false))

(fn TickGlide
  (params (DeltaSeconds :type Float%20%28single-precision%29))
  (bind _owningcharacter (CallFunction|GetOwningCharacter))
  (bind _glidecurve (Variables|Private|GetGlideCurve))
  (bind (_mintime _maxtime) (Math|Curves|GetTimeRange _glidecurve))
  (bind _charactermovement (Variables|/Script/Engine.Character|GetCharacterMovement _owningcharacter))
  (bind _output_get (Variables|Default|SetGlideTimer (+ (Variables|Default|GetGlideTimer) DeltaSeconds)))
  (if (Math|Float|InRange(Float) _output_get _mintime _maxtime)
    (Variables|/Script/Engine.MovementComponent|SetVelocity _charactermovement (Math|Vector|MakeVector (.x (Variables|/Script/Engine.MovementComponent|GetVelocity _charactermovement)) (.y (Variables|/Script/Engine.MovementComponent|GetVelocity _charactermovement)) (Math|Float|Max(Float) (.z (Variables|/Script/Engine.MovementComponent|GetVelocity _charactermovement)) (Math|Curves|GetFloatValue (Variables|Private|GetGlideCurve) (Variables|Default|GetGlideTimer)))))
    (else
      (Private|EndGlide))))

(fn StopJumping
  (Private|EndGlide)
  (|CallParentFunction))