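; BP_JumpComponentBase is a base component that provides jump behavior for a Character owner.
; On BeginPlay it caches the owning Character, or destroys itself if the owner is not a Character.
; Jump and StopJumping forward to the Character's built-in functions, and a getter exposes the cached owner.
; OnLanded and GetJumpCount are empty stubs in this base.
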(event EventBeginPlay
  (bind _ascharacter (Utilities|Casting|CastToCharacter (Components|GetOwner))
    (:then
      (Variables|Private|SetOwningCharacter _ascharacter))
    (:CastFailed
      (Components|DestroyComponent))))

(event EventTick
  (params (DeltaSeconds :type Float%20%28single-precision%29)))

(fn Jump
  (Character|Jump (Variables|Private|GetOwningCharacter)))

(fn StopJumping
  (Character|StopJumping (Variables|Private|GetOwningCharacter)))

(fn OnLanded)

(fn GetJumpCount)

(fn GetOwningCharacter
  (return (Variables|Private|GetOwningCharacter)))